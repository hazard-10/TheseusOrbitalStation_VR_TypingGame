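; VR keyboard component that types characters through hand movement around the headset.
; Each tick, the camera-to-controller vector's horizontal angle from an anchor highlights one key panel across an evenly divided arc.
; Left thumbstick Y switches each panel's active key, and the Y button recaptures the anchor.
; Crossing a vertical angle threshold sends the highlighted key to the text display once, using a lock until the angle returns.
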(event EventBeginPlay
  (Utilities|FlowControl|Sequence
    (:then_0
      (bind _returnvalue (Actor|GetActorOfClass "/Game/VRTemplate/Blueprints/VRPawn.VRPawn_C"))
      (Variables|Default|SetVRPawnRef _returnvalue)
      (CallFunction|CalculateAngleRanges)
      (CallFunction|ResetAnchorAxis)
      (bind _returnvalue_2 (Actor|GetActorOfClass "/Game/Blueprints/Actors/TestUIPanel.TestUIPanel_C"))
      (bind _astest_uiwidget (Utilities|Casting|CastToTestUIWidget (UserInterface|GetUserWidgetObject (Variables|/Game/Blueprints/Actors/TestUIPanel.TestUIPanel_C|GetWidget _returnvalue_2))))
      (Variables|Default|SetTestingPanel _astest_uiwidget)
      (Input|EnableInput (Components|GetOwner) (Game|GetPlayerController 0)))
    (:then_1
      (Utilities|FlowControl|Delay 0.2)
      (bind _returnvalue_3 (Actor|GetActorOfClass "/Game/Blueprints/Actors/TextDisplayBP.TextDisplayBP_C"))
      (bind _astext_display (Utilities|Casting|CastToTextDisplay (UserInterface|GetUserWidgetObject (Variables|/Game/Blueprints/Actors/TextDisplayBP.TextDisplayBP_C|GetWidget _returnvalue_3))))
      (Variables|Default|SetTextDisplayPanel _astext_display))))

(event EventTick
  (params (DeltaSeconds :type Float%20%28single-precision%29))
  (CallFunction|ProcessControllerRotation))

(event Input|ActionEvents|InputActionLeftControlPressY
  (params (Key :type Key%20Structure))
  ;[0 0 0] Processing inputs
  (:Pressed
    (CallFunction|ResetAnchorAxis)))

(event Input|AxisEvents|InputAxisMovementAxisLeft_Y
  (params (AxisValue :type Float%20%28single-precision%29))
  ;[0 0 0] Processing inputs
  (CallFunction|ProcessAxisData AxisValue))

(fn ProcessControllerRotation
  (bind _anchoraxis (Variables|Default|GetAnchorAxis))
  (bind _motioncontrollerdata (Class|HeadMountedDisplayFunctionLibrary|GetMotionControllerData (Variables|Default|GetVRPawnRef) (Variables|Default|GetControlHand)))
  (Utilities|FlowControl|Sequence
    (:then_0
      (bind _angle (CallFunction|AngleBetween _anchoraxis (Utilities|ClearZAxis (- (.GripPosition (Utilities|Struct|BreakXRMotionControllerData _motioncontrollerdata)) (Transformation|GetWorldLocation (Variables|/Game/VRTemplate/Blueprints/VRPawn.VRPawn_C|GetCamera (Variables|Default|GetVRPawnRef))))) "0, 0,1.000000"))
      (bind _currentpanel (CallFunction|GetPanelbyAngle _angle))
      (bind _astest_uipanel (Utilities|Casting|CastToTestUIPanel _currentpanel))
      (bind _astest_uiwidget (Utilities|Casting|CastToTestUIWidget (UserInterface|GetUserWidgetObject (Variables|/Game/Blueprints/Actors/TestUIPanel.TestUIPanel_C|GetWidget _astest_uipanel))))
      (Variables|/Game/Blueprints/Actors/TestUIWidget.TestUIWidget_C|SetHighlighted _astest_uiwidget true)
      (Variables|Default|SethighlightedKey (Variables|/Game/Blueprints/Actors/TestUIWidget.TestUIWidget_C|GethighlightedKey _astest_uiwidget)))
    (:then_1
      (bind _angle_2 (CallFunction|AngleBetween _anchoraxis (Utilities|ClearYAxisRelitivetoAnchor (- (.GripPosition (Utilities|Struct|BreakXRMotionControllerData _motioncontrollerdata)) (Transformation|GetWorldLocation (Variables|/Game/VRTemplate/Blueprints/VRPawn.VRPawn_C|GetCamera (Variables|Default|GetVRPawnRef))))) "0,1.000000, 0"))
      (Utilities|FlowControl|Sequence
        (:then_0
          (if (< _angle_2 (+ (Variables|Default|GetInputThresholdAngle) (Variables|Default|GetAnchorZAngle)))
            (if (not (Variables|Default|GetInputLock))
              (Variables|Default|SetInputLock true)
              (Default|UpdateText (Variables|Default|GetTextDisplayPanel) (Variables|Default|GethighlightedKey)))
            (else
              (Variables|Default|SetInputLock false))))
        (:then_1
          (Default|UpdateAngle (Variables|Default|GetTextDisplayPanel) _angle_2)
          (CallFunction|DrawDebugArrowSupport (Utilities|ClearYAxisRelitivetoAnchor (- (.GripPosition (Utilities|Struct|BreakXRMotionControllerData _motioncontrollerdata)) (Transformation|GetWorldLocation (Variables|/Game/VRTemplate/Blueprints/VRPawn.VRPawn_C|GetCamera (Variables|Default|GetVRPawnRef))))) (Class|KismetMathLibrary|LinearColortoRGBE "(R=0.942708,G=0.093289,B=0.093289,A=1.000000)") 0.0))))))

(fn CalculateAngleRanges
  (Variables|Default|SetAnglePerPanel (/ (Variables|Default|GetTotalAngleRange) (Utilities|Array|Length (Variables|Default|GetKeyPanels)))))

(fn GetPanelbyAngle
  (params (Angle :type Float%20%28double-precision%29))
  (bind _angleperpanel (Variables|Default|GetAnglePerPanel))
  (bind _keypanels (Variables|Default|GetKeyPanels))
  (while (< (LocalVariables|GetCurrentIndex) (Utilities|Array|Length (Variables|Default|GetKeyPanels)))
    (LocalVariables|SetCurrentIndex (+ (LocalVariables|GetCurrentIndex) 1))
    (if (< Angle (- (* (LocalVariables|GetCurrentIndex) _angleperpanel) (* _angleperpanel (/ (Utilities|Array|Length (Variables|Default|GetKeyPanels)) 2))))
      (for _array_element (Variables|Default|GetKeyPanels)
        (bind _astest_uipanel (Utilities|Casting|CastToTestUIPanel _array_element))
        (bind _astest_uiwidget (Utilities|Casting|CastToTestUIWidget (UserInterface|GetUserWidgetObject (Variables|/Game/Blueprints/Actors/TestUIPanel.TestUIPanel_C|GetWidget _astest_uipanel))))
        (Variables|/Game/Blueprints/Actors/TestUIWidget.TestUIWidget_C|SetHighlighted _astest_uiwidget false))
      (return (Utilities|Array|Get(acopy) (Variables|Default|GetKeyPanels) (- (LocalVariables|GetCurrentIndex) 1)))))
  (return (Utilities|Array|Get(acopy) _keypanels (Utilities|Array|LastIndex _keypanels))))

(fn ResetAnchorAxis
  (bind _vrpawnref (Variables|Default|GetVRPawnRef))
  (bind _motioncontrollerdata (Class|HeadMountedDisplayFunctionLibrary|GetMotionControllerData _vrpawnref (Variables|Default|GetControlHand)))
  (bind _output_get (Variables|Default|SetAnchorAxis (Utilities|ClearZAxis (- (.GripPosition (Utilities|Struct|BreakXRMotionControllerData _motioncontrollerdata)) (Transformation|GetWorldLocation (Variables|/Game/VRTemplate/Blueprints/VRPawn.VRPawn_C|GetCamera _vrpawnref))))))
  (CallFunction|DrawDebugArrowSupport _output_get (Class|KismetMathLibrary|LinearColortoRGBE "(R=1.000000,G=0.806257,B=0.056156,A=1.000000)") 5.0)
  (bind _angle (CallFunction|AngleBetween _output_get (- (.GripPosition (Utilities|Struct|BreakXRMotionControllerData _motioncontrollerdata)) (Transformation|GetWorldLocation (Variables|/Game/VRTemplate/Blueprints/VRPawn.VRPawn_C|GetCamera _vrpawnref))) "0,1.000000, 0"))
  (Variables|Default|SetAnchorZAngle _angle))

(fn AngleBetween
  (params (Vec1 :type Vector) (Vec2 :type Vector) (Normal :type Vector))
  (bind _returnvalue (Math|Vector|Normalize Vec2))
  (bind _returnvalue_2 (Math|Vector|Normalize Vec1))
  (return (Class|KismetMathLibrary|DegAtan (/ (Math|Vector|DotProduct (Math|Vector|CrossProduct _returnvalue_2 _returnvalue) Normal) (Math|Vector|DotProduct _returnvalue_2 _returnvalue)))))

(fn ProcessAxisData
  (params (YAxis :type Float%20%28double-precision%29))
  (Utilities|FlowControl|Sequence
    (:then_0
      (if (> YAxis 0.0)
        (CallFunction|SwitchKeyIndex)
        (else
          (CallFunction|SwitchKeyIndex 1))))
    (:then_1
      (if (< YAxis 0.0)
        (CallFunction|SwitchKeyIndex 2)))))

(fn SwitchKeyIndex
  (params (Index :type Integer))
  (for _array_element (Variables|Default|GetKeyPanels)
    (bind _astest_uipanel (Utilities|Casting|CastToTestUIPanel _array_element))
    (bind _astest_uiwidget (Utilities|Casting|CastToTestUIWidget (UserInterface|GetUserWidgetObject (Variables|/Game/Blueprints/Actors/TestUIPanel.TestUIPanel_C|GetWidget _astest_uipanel))))
    (Default|UpdateHighlightKey _astest_uiwidget Index)))

(fn DrawDebugArrowSupport
  (params (Direction :type Vector) (Color :type Color%20Structure) (Duration :type Float%20%28double-precision%29))
  (bind _vrpawnref (Variables|Default|GetVRPawnRef))
  (bind _camera (Variables|/Game/VRTemplate/Blueprints/VRPawn.VRPawn_C|GetCamera _vrpawnref))
  (bind _returnvalue (Transformation|GetWorldLocation _camera))
  (Rendering|Debug|DrawDebugArrow _returnvalue (+ _returnvalue (* Direction "100.000000,100.000000,100.000000")) 3.0 (Math|Conversions|ToLinearColor(Color) Color) Duration 3.0))