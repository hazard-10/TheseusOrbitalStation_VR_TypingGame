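; BP_StoryDisplay is an actor that builds up story sentences word by word in a StoryDisplayBox widget, framed by four border cubes.
; changeWidgetEvent strips highlight tags by substring offsets, appends the word and flashes the border.
; A trailing period calls CallOnLineFinish, shows the border longer, then clears the text.
; ChangeWidgetText is a similar function that busy-waits on the Tick counter, which cannot advance inside the loop.
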(event Custom|changeWidgetEvent
  (params (newword :type String))
  (bind _returnvalue (Utilities|String|Len newword))
  (bind _returnvalue_2 (- _returnvalue 15))
  (bind _returnvalue_3 (- _returnvalue 4))
  (bind _returnvalue_4 (Utilities|String|GetSubstring newword 11 _returnvalue_2))
  (bind _returnvalue_5 (Utilities|String|GetSubstring newword _returnvalue_3))
  (bind _returnvalue_6 (Utilities|String|Append _returnvalue_4 _returnvalue_5))
  (bind _returnvalue_7 (Utilities|String|GetCharacterArrayfromString _returnvalue_6))
  (bind _asstory_display_box (Utilities|Casting|CastToStoryDisplayBox (UserInterface|GetUserWidgetObject (Variables|Default|GetWidget))))
  (CallFunction|ShowBorder true)
  (Default|UpdateContent _asstory_display_box (Utilities|String|Append (Variables|/Game/p3/GameUI/StoryDisplayBox.StoryDisplayBox_C|Getcontent _asstory_display_box) "  " _returnvalue_6))
  (Utilities|FlowControl|Delay 1.0)
  (CallFunction|ShowBorder false)
  (if (Utilities|Enum|Equal(Enum) (Utilities|Array|Get(acopy) _returnvalue_7 (- (Utilities|Array|Length _returnvalue_7) 1)) ".")
    (Default|CallOnLineFinish)
    (CallFunction|ShowBorder true)
    (Utilities|FlowControl|Delay 5.0)
    (CallFunction|ShowBorder false)
    (Default|UpdateContent _asstory_display_box)))

(event EventBeginPlay
  (CallFunction|ShowBorder false))

(event Collision|EventActorBeginOverlap
  (params (OtherActor :type Actor%20Object%20Reference)))

(event EventTick
  (params (DeltaSeconds :type Float%20%28single-precision%29))
  (Variables|Default|Settimer (+ (Variables|Default|Gettimer) 1)))

(fn ConstructionScript)

(fn ShowBorder
  (params (show :type Boolean))
  (Rendering|SetVisibility (Variables|Default|GetCube3) show true)
  (Rendering|SetVisibility (Variables|Default|GetCube2) show true)
  (Rendering|SetVisibility (Variables|Default|GetCube1) show true)
  (Rendering|SetVisibility (Variables|Default|GetCube) show true))

(fn ChangeWidgetText
  (params (new_word :type String))
  (bind _returnvalue (Utilities|String|Len new_word))
  (bind _returnvalue_2 (- _returnvalue 15))
  (bind _returnvalue_3 (- _returnvalue 1))
  (bind _returnvalue_4 (Utilities|String|GetSubstring new_word 11 _returnvalue_2))
  (bind _returnvalue_5 (Utilities|String|GetSubstring new_word _returnvalue_3))
  (bind _returnvalue_6 (Utilities|String|Append _returnvalue_4 _returnvalue_5))
  (bind _returnvalue_7 (Utilities|String|GetCharacterArrayfromString _returnvalue_6))
  (Development|PrintString _returnvalue_6)
  (bind _asstory_display_box (Utilities|Casting|CastToStoryDisplayBox (UserInterface|GetUserWidgetObject (Variables|Default|GetWidget))))
  (CallFunction|ShowBorder true)
  (LocalVariables|SettmpTimer (Variables|Default|Gettimer))
  (Default|UpdateContent _asstory_display_box (Utilities|String|Append (Variables|/Game/p3/GameUI/StoryDisplayBox.StoryDisplayBox_C|Getcontent _asstory_display_box) "" _returnvalue_6))
  (while (> (LocalVariables|GettmpTimer) (- (Variables|Default|Gettimer) 5))
    _)
  (CallFunction|ShowBorder false)
  (if (Utilities|Enum|Equal(Enum) (Utilities|Array|Get(acopy) _returnvalue_7 (- (Utilities|Array|Length _returnvalue_7) 1)) ".")
    (Default|UpdateContent _asstory_display_box)))