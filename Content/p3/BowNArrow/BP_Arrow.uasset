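; BP_Arrow is a homing arrow projectile that destroys the demon it targets on contact.
; Each tick it faces a valid Target and offsets itself locally along its forward vector, at a speed proportional to remaining distance.
; Overlapping the Target spawns an explosion, destroys the arrow and calls DestroyDemon on DemonManager.
; FindNewTarget can copy DemonManager's TargetDemon, but its event-graph call is disconnected.
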(event OnComponentBeginOverlap(StaticMeshComponent)
  (params (OverlappedComponent :type Primitive%20Component%20Object%20Reference) (OtherActor :type Actor%20Object%20Reference) (OtherComp :type Primitive%20Component%20Object%20Reference) (OtherBodyIndex :type Integer) (bFromSweep :type Boolean) (SweepResult :type Hit%20Result%20Structure%20%28by%20ref%29))
  (if (== OtherActor (Variables|Default|Gettarget))
    (Game|SpawnActorfromClass "/Game/p3/VFX/Explosion/P_Explosion_Big_A_Converted_Blueprint.P_Explosion_Big_A_Converted_Blueprint_C" (Transformation|GetActorTransform self) "Undefined" 0 0)
    (Actor|DestroyActor)
    (Default|DestroyDemon (Variables|Default|Getdemon_manager) (Variables|Default|Gettarget))))

(event EventTick
  (params (DeltaSeconds :type Float%20%28single-precision%29))
  (Utilities|IsValid (Variables|Default|Gettarget)
    (:Is%20Valid
      (Transformation|SetActorRotation (Math|Rotator|FindLookatRotation (Transformation|GetActorLocation) (.Location (Math|Transform|BreakTransform (Transformation|GetActorTransform (Variables|Default|Gettarget))))))
      (Variables|Default|Setarrow_speed (/ (Transformation|GetDistanceTo (Variables|Default|Gettarget)) 0.5))
      (Transformation|AddActorLocalOffset (* (Transformation|GetActorForwardVector) (* (Variables|Default|Getarrow_speed) (Utilities|Time|GetWorldDeltaSeconds))) false false))))

(fn ConstructionScript)

(fn FindNewTarget
  (Variables|Default|Settarget (Variables|/Game/p3/manage_all_demons.manage_all_demons_C|Gettarget_demon (Variables|Default|Getdemon_manager))))