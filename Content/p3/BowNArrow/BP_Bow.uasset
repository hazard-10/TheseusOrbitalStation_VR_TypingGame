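; BP_Bow is the player's weapon in a typing game, firing at demons as their words are typed.
; With no target, Tick picks the first demon in the manager's list whose word starts with the latest input character.
; Each matching letter updates the arrow widget; intermediate letters also trigger key VFX, spawn a stone and update the demon's text.
; Completing the word spawns an arrow and clears the target.
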(event EventBeginPlay
  (Utilities|FlowControl|Sequence
    (:then_0
      (bind _outactors (Actor|GetAllActorswithTag "demon_manager"))
      (Variables|Default|Setdemon_manager (Actor|GetComponentbyClass (Utilities|Array|Get(acopy) _outactors) "/Game/p3/manage_all_demons.manage_all_demons_C")))
    (:then_1
      (bind _returnvalue (Actor|GetActorOfClass "/Game/KeyboardDesigns/SpeedTestLevel/BPGameManager.BPGameManager_C"))
      (Variables|Default|Setgame_manager _returnvalue))
    (:then_2
      (CallFunction|UpdateTargetString))))

(event EventTick
  (params (DeltaSeconds :type Float%20%28single-precision%29))
  (if (Variables|Default|Gethas_target_demon)
    (CallFunction|RecordString :!label _label)
    (if (Utilities|Enum|Equal(Enum) (Variables|Default|Getcurrent_string) (Variables|Default|Gettarget_string))
      (CallFunction|ShootArrow)
      ;[1 1 1] After arrow is shot, before new demon is found, target string is empty
      (Variables|Default|Setcurrent_string "")
      (Variables|Default|Settarget_string "")
      (CallFunction|UpdateTargetString))
    (else
      (bind _found (CallFunction|FindTargetDemon))
      (if _found
        (goto _label)))))

(fn ConstructionScript)

(fn ShootArrow
  (params (target_actor :type Actor%20Object%20Reference))
  (bind _returnvalue (Game|SpawnActorfromClass "/Game/p3/BowNArrow/BP_Arrow.BP_Arrow_C" (Transformation|GetActorTransform) "Undefined" 0 0))
  (Variables|/Game/p3/BowNArrow/BP_Arrow.BP_Arrow_C|Settarget _returnvalue target_actor)
  (Variables|/Game/p3/BowNArrow/BP_Arrow.BP_Arrow_C|Setdemon_manager _returnvalue (Variables|Default|Getdemon_manager))
  (Variables|Default|Sethas_target_demon false))

(fn RecordString
  (bind _game_manager (Variables|Default|Getgame_manager))
  (bind _demon_manager (Variables|Default|Getdemon_manager))
  (bind _inputtext (Variables|/Game/KeyboardDesigns/SpeedTestLevel/BPGameManager.BPGameManager_C|GetInputText _game_manager))
  (bind _target_demon (Variables|/Game/p3/manage_all_demons.manage_all_demons_C|Gettarget_demon _demon_manager))
  (bind _returnvalue (Utilities|String|GetCharacterArrayfromString _inputtext))
  (bind _returnvalue_2 (Utilities|Array|Length _returnvalue))
  (bind _returnvalue_3 (- _returnvalue_2 1))
  (if (Utilities|Enum|Equal(Enum) (Utilities|Array|Get(acopy) (Utilities|String|GetCharacterArrayfromString (Variables|Default|Gettarget_string)) (Utilities|String|Len (Variables|Default|Getcurrent_string))) (Utilities|Array|Get(acopy) _returnvalue _returnvalue_3))
    (bind _output_get (Variables|Default|Setcurrent_string (Utilities|String|Append (Variables|Default|Getcurrent_string) (Utilities|Array|Get(acopy) _returnvalue _returnvalue_3))))
    (bind _asarrow_widget (Utilities|Casting|CastToArrowWidget (UserInterface|GetUserWidgetObject (Variables|Default|GetWidget))))
    (bind _new_text (Default|HighlightCharacter _asarrow_widget (Utilities|String|Len _output_get)))
    (if (not (Utilities|Enum|Equal(Enum) (Variables|Default|Getcurrent_string) (Variables|Default|Gettarget_string)))
      (Default|KeyPressVFX (Variables|/Game/KeyboardDesigns/SpeedTestLevel/BPGameManager.BPGameManager_C|GetLastKeyPressActor (Variables|Default|Getgame_manager)) _target_demon)
      (CallFunction|ShootStone)
      (bind _asbp_demon (Utilities|Casting|CastToBP_demon _target_demon))
      (Variables|/Game/p3/demon/BP_demon.BP_demon_C|Setword _asbp_demon (Utilities|String|ToString(Text) _new_text))
      (Default|SetDemonText _asbp_demon))))

(fn UpdateTargetString
  (bind _asarrow_widget (Utilities|Casting|CastToArrowWidget (UserInterface|GetUserWidgetObject (Variables|Default|GetWidget))))
  (Default|SpawnNewString _asarrow_widget (Variables|Default|Gettarget_string)))

(fn FindTargetDemon
  (bind _game_manager (Variables|Default|Getgame_manager))
  (bind _inputtext (Variables|/Game/KeyboardDesigns/SpeedTestLevel/BPGameManager.BPGameManager_C|GetInputText _game_manager))
  (bind _returnvalue (Utilities|String|GetCharacterArrayfromString _inputtext))
  (bind _array_element (Utilities|Array|ForEachLoopwithBreak (Variables|/Game/p3/manage_all_demons.manage_all_demons_C|Getdemon_list (Variables|Default|Getdemon_manager)))
    (:LoopBody
      (bind _asbp_demon (Utilities|Casting|CastToBP_demon _array_element))
      (if (Utilities|Enum|Equal(Enum) (Utilities|Array|Get(acopy) (Utilities|String|GetCharacterArrayfromString (Variables|/Game/p3/demon/BP_demon.BP_demon_C|Getword _asbp_demon))) (Utilities|Array|Get(acopy) _returnvalue (- (Utilities|Array|Length _returnvalue) 1)))
        (Development|PrintString "find demon")
        (Variables|/Game/p3/manage_all_demons.manage_all_demons_C|Settarget_demon (Variables|Default|Getdemon_manager) _array_element)
        (Variables|Default|Sethas_target_demon true)
        (bind _output_get (Variables|Default|Settarget_string (Variables|/Game/p3/demon/BP_demon.BP_demon_C|Getword _asbp_demon)))
        (Development|PrintString _output_get)
        (CallFunction|UpdateTargetString)
        (return true)))
    (:Completed
      (return false))))

(fn ShootStone
  (params (targetActor :type Actor%20Object%20Reference))
  (bind _returnvalue (Game|SpawnActorfromClass "/Game/p3/stone/BP_stone.BP_stone_C" (Transformation|GetActorTransform) "Undefined" 0 0))
  (Development|PrintString "spawn stone")
  (Variables|/Game/p3/stone/BP_stone.BP_stone_C|Settarget _returnvalue targetActor)
  (Variables|/Game/p3/stone/BP_stone.BP_stone_C|Setdemon_manager _returnvalue (Variables|Default|Getdemon_manager)))