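; BP_stone is a homing projectile that flies at a demon target and, on overlapping it, triggers that demon's hit effect and destroys itself.
; Each tick it turns toward the target and moves forward by Speed, calling FindNewTarget when the target is invalid.
; FindNewTarget is empty, with its DemonManager target lookup left disconnected.
; SetSpeed, not called here, derives Speed from target distance for a one-second flight.
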(event OnComponentBeginOverlap(StaticMeshComponent)
  (params (OverlappedComponent :type Primitive%20Component%20Object%20Reference) (OtherActor :type Actor%20Object%20Reference) (OtherComp :type Primitive%20Component%20Object%20Reference) (OtherBodyIndex :type Integer) (bFromSweep :type Boolean) (SweepResult :type Hit%20Result%20Structure%20%28by%20ref%29))
  (bind _target (Variables|Default|Gettarget))
  (if (== OtherActor _target)
    (bind _asbp_demon (Utilities|Casting|CastToBP_demon _target))
    (Default|UpdateHitEffect _asbp_demon)
    (Actor|DestroyActor)))

(event EventBeginPlay)

(event EventTick
  (params (DeltaSeconds :type Float%20%28single-precision%29))
  (Utilities|IsValid (Variables|Default|Gettarget)
    (:Is%20Valid
      _)
    (:Is%20Not%20Valid
      (CallFunction|FindNewTarget)
      (Utilities|IsValid (Variables|Default|Gettarget)
        (:Is%20Valid
          _))))
  (Transformation|SetActorRotation (Math|Rotator|FindLookatRotation (Transformation|GetActorLocation) (.Location (Math|Transform|BreakTransform (Transformation|GetActorTransform (Variables|Default|Gettarget))))))
  (Transformation|AddActorLocalOffset (* (Transformation|GetActorForwardVector) (* (Variables|Default|Getspeed) (Utilities|Time|GetWorldDeltaSeconds))) false false))

(fn ConstructionScript)

(fn FindNewTarget)

(fn SetSpeed
  (bind _target (Variables|Default|Gettarget))
  (Utilities|IsValid _target
    (:Is%20Valid
      (Variables|Default|Setspeed (/ (Transformation|GetDistanceTo _target) 1.0)))))