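; Actor that builds a spline path from a list of world-space points and lays spline meshes along it.
; On BeginPlay it passes two hardcoded test points to LoadSpline, which moves the first two spline points, appends any others and prints debug output.
; LoadMesh then adds one SplineMeshComponent per segment, using each end's local location and tangent so the meshes follow the curve.
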(event EventBeginPlay
  (CallFunction|LoadSpline (Utilities|Array|MakeArray (Math|Vector|MakeVector 0.0 0.0 0.0) (Math|Vector|MakeVector 1e+02 2e+01 1e+01))))

(event Collision|EventActorBeginOverlap
  (params (OtherActor :type Actor%20Object%20Reference)))

(event EventTick
  (params (DeltaSeconds :type Float%20%28single-precision%29)))

(fn ConstructionScript)

(fn LoadSpline
  (params (NewParam :type Array%20of%20Vectors))
  (LocalVariables|SetCoordinates NewParam)
  (for _array_element (LocalVariables|GetCoordinates)
    (Development|PrintString (Utilities|String|Append (Utilities|String|ToString(Vector) _array_element) "zzzz")))
  (Spline|SetLocationatSplinePoint (Variables|Default|GetSpline1) 0 (Utilities|Array|Get(acopy) (LocalVariables|GetCoordinates)) "World" true)
  (Spline|SetLocationatSplinePoint (Variables|Default|GetSpline1) 1 (Utilities|Array|Get(acopy) (LocalVariables|GetCoordinates) 1) "World" true)
  (Development|PrintString (Utilities|String|Append "spl before loading has" (Utilities|String|ToString(Integer) (Spline|GetNumberOfSplinePoints (Variables|Default|GetSpline1)))))
  (for _index (range 2 (- (Utilities|Array|Length (LocalVariables|GetCoordinates)) 1))
    (Spline|AddSplinePoint (Variables|Default|GetSpline1) (Utilities|Array|Get(acopy) (LocalVariables|GetCoordinates) _index) "World" true))
  (Development|PrintString (Utilities|String|Append "spl before exit has" (Utilities|String|ToString(Integer) (Spline|GetNumberOfSplinePoints (Variables|Default|GetSpline1)))))
  (CallFunction|LoadMesh))

(fn LoadMesh
  (bind _spline1 (Variables|Default|GetSpline1))
  (for _index (range 0 (- (Spline|GetNumberOfSplinePoints (Variables|Default|GetSpline1)) 2))
    (bind _returnvalue (AddComponent|AddSplineMeshComponent false))
    (SplineMesh|SetStartandEnd _returnvalue (.Location (Spline|GetLocationandTangentatSplinePoint _spline1 _index "Local")) (.Tangent (Spline|GetLocationandTangentatSplinePoint _spline1 _index "Local")) (.Location (Spline|GetLocationandTangentatSplinePoint _spline1 (+ _index 1) "Local")) (.Tangent (Spline|GetLocationandTangentatSplinePoint _spline1 (+ _index 1) "Local")) true :!class /Script/Engine.SplineMeshComponent)))