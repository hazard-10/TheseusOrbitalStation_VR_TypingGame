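; Analytics manager actor that shows recorded left and right location data as spline paths alongside a widget.
; ShowAnalytics reveals the widget, hides the environment actors and redraws both splines.
; DrawSpline replaces any existing BP_SplineDrawPath actors and feeds them fixed-offset coordinates from BPDataRecordManager, found on BeginPlay.
; Next and previous calls only step the record manager without redrawing; closing hides the widget and destroys the splines, while ShowEnv separately restores the environment.
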(event EventBeginPlay
  (bind _returnvalue (Actor|GetActorOfClass "/Game/p3/BPDataRecordManager.BPDataRecordManager_C"))
  (Variables|Default|SetDM _returnvalue))

(event Collision|EventActorBeginOverlap
  (params (OtherActor :type Actor%20Object%20Reference)))

(event EventTick
  (params (DeltaSeconds :type Float%20%28single-precision%29)))

(fn ConstructionScript)

(fn ShowEnv
  (for _array_element (Variables|Default|GetEnv)
    (Rendering|SetActorHiddenInGame _array_element false)))

(fn HideEnv
  (for _array_element (Variables|Default|GetEnv)
    (Rendering|SetActorHiddenInGame _array_element true)))

(fn ShowAnalytics
  (Rendering|SetVisibility (Variables|Default|GetWidget) true false)
  (CallFunction|HideEnv)
  (CallFunction|DrawSpline))

(fn DrawSpline
  (CallFunction|ClearSpline)
  (bind _returnvalue (Game|SpawnActorfromClass "/Game/p3/analytics/BP_SplineDrawPath.BP_SplineDrawPath_C" (Math|Transform|MakeTransform "0, 0, 0" "0, 0, 0" "1.000000,1.000000,1.000000") "Undefined" 0 0))
  (Variables|Default|SetLeftSpline _returnvalue)
  (bind _returnvalue_2 (Game|SpawnActorfromClass "/Game/p3/analytics/BP_SplineDrawPath.BP_SplineDrawPath_C" (Math|Transform|MakeTransform "0, 0, 0" "0, 0, 0" "1.000000,1.000000,1.000000") "Undefined" 0 0))
  (Variables|Default|SetRightSpline _returnvalue_2)
  (bind (_target_letter _left_location_list _right_location_list) (Default|GetDataforAnalysis (Variables|Default|GetDM)))
  (bind _out (CallFunction|(Private)SetCursorTransform _left_location_list))
  (bind _out_2 (CallFunction|(Private)SetCursorTransform _right_location_list))
  (Variables|/Game/p3/analytics/BP_SplineDrawPath.BP_SplineDrawPath_C|SetCoordinates (Variables|Default|GetLeftSpline) _out)
  (Variables|/Game/p3/analytics/BP_SplineDrawPath.BP_SplineDrawPath_C|SetCoordinates (Variables|Default|GetRightSpline) _out_2))

(fn CloseUIandDestorySpline
  (Rendering|SetVisibility (Variables|Default|GetWidget) false false)
  (Actor|DestroyActor (Variables|Default|GetLeftSpline))
  (Actor|DestroyActor (Variables|Default|GetRightSpline)))

(fn (Private)SetCursorTransform
  (params (in :type Array%20of%20Vectors))
  (for _array_element in
    (Utilities|Array|Add (LocalVariables|Getans) (+ _array_element "6.000000,0.000000,4.000000")))
  (return (LocalVariables|Getans)))

(fn NextSpline
  (Default|MovetoNext (Variables|Default|GetDM)))

(fn PrevSpline
  (Default|MovetoPrevious (Variables|Default|GetDM)))

(fn ClearSpline
  (Actor|DestroyActor (Variables|Default|GetLeftSpline))
  (Actor|DestroyActor (Variables|Default|GetRightSpline)))