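; Blueprint that draws a path through a supplied list of coordinates as a chain of spline meshes.
; LoadCoordinates stores the points, then calls LoadSpline, which moves the first two spline points and appends the rest in world space.
; LoadMesh then adds a spline mesh component per segment, choosing one of two templates by IsLeft, and fits it to the segment's local-space locations and tangents.
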(fn ConstructionScript)

(fn LoadSpline
  (bind _coordinates (Variables|Default|GetCoordinates))
  (for _array_element (Variables|Default|GetCoordinates)
    _)
  (Spline|SetLocationatSplinePoint (Variables|Default|GetSpline1) 0 (Utilities|Array|Get(acopy) (Variables|Default|GetCoordinates)) "World" true)
  (Spline|SetLocationatSplinePoint (Variables|Default|GetSpline1) 1 (Utilities|Array|Get(acopy) (Variables|Default|GetCoordinates) 1) "World" true)
  (for _index (range 2 (- (Utilities|Array|Length _coordinates) 1))
    (Spline|AddSplinePoint (Variables|Default|GetSpline1) (Utilities|Array|Get(acopy) _coordinates _index) "World" true)))

(fn LoadMesh
  (bind _spline1 (Variables|Default|GetSpline1))
  (for _index (range 0 (- (Spline|GetNumberOfSplinePoints (Variables|Default|GetSpline1)) 2))
    (if (Variables|Default|GetisLeft)
      (bind _returnvalue (AddComponent|AddSplineMeshComponent false))
      (else
        (bind _returnvalue_2 (AddComponent|AddSplineMeshComponent false))))
    (SplineMesh|SetStartandEnd _returnvalue (.Location (Spline|GetLocationandTangentatSplinePoint _spline1 _index "Local")) (.Tangent (Spline|GetLocationandTangentatSplinePoint _spline1 _index "Local")) (.Location (Spline|GetLocationandTangentatSplinePoint _spline1 (+ _index 1) "Local")) (.Tangent (Spline|GetLocationandTangentatSplinePoint _spline1 (+ _index 1) "Local")) true :!class /Script/Engine.SplineMeshComponent)))

(fn LoadCoordinates
  (params (coor :type Array%20of%20Vectors))
  (Utilities|Array|Clear (Variables|Default|GetCoordinates))
  (Variables|Default|SetCoordinates coor)
  (CallFunction|LoadSpline)
  (CallFunction|LoadMesh))