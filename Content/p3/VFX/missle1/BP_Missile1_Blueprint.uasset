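; BP_Missile1_Blueprint is a missile VFX actor whose Niagara effect follows a target actor, Aim.
; Each Tick writes Aim's location into the Niagara "aim" vector variable, or destroys the actor if Aim is invalid.
; BeginPlay caps its lifetime at three seconds with a delayed destroy.
; The Blueprint itself contains no movement or damage logic.
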(event EventBeginPlay
  (Utilities|FlowControl|Delay 3.0)
  (Actor|DestroyActor))

(event EventTick
  (params (DeltaSeconds :type Float%20%28single-precision%29))
  (bind _aim (Variables|Default|Getaim))
  (if (Utilities|IsValid _aim)
    (Niagara|SetNiagaraVariable(Vector3) (Variables|NiagaraActor|GetNiagaraComponent) "aim" (Transformation|GetActorLocation _aim))
    (else
      (Actor|DestroyActor))))

(fn ConstructionScript)