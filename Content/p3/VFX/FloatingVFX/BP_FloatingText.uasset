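; BP_FloatingText is a Niagara floating-letter actor that can drift toward a BP_TextBox in the level.
; ShowLetter maps a letter from A to Z to its texture and sets it on the Niagara "user.Alphabet" parameter.
; BeginPlay caches the first BP_TextBox, and while ShouldMove is set, Tick applies the unit direction times delta seconds as a local offset, without an arrival check.
; The overlap handler is empty and never bound.
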(event Custom|OnActorBeginOverlap_Event
  (params (OverlappedActor :type Actor%20Object%20Reference) (OtherActor :type Actor%20Object%20Reference)))

(event EventBeginPlay
  (bind _outactors (Actor|GetAllActorsOfClass "/Game/p3/BP_TextBox.BP_TextBox_C"))
  (Variables|Default|Settextbox_ref (Utilities|Array|Get(acopy) _outactors)))

(event EventTick
  (params (DeltaSeconds :type Float%20%28single-precision%29))
  (if (Variables|Default|GetshouldMove)
    ;[1 1 1] move towards textbox location if havent reached
    (Transformation|AddActorLocalOffset (* (Math|Vector|GetUnitDirection(Vector) (.location (Transformation|GetActorTransform)) (Transformation|GetActorLocation (Variables|Default|Gettextbox_ref))) (Utilities|Time|GetWorldDeltaSeconds)) false false)))

(fn ConstructionScript)

(fn ShowLetter
  (params (letter :type String))
  (switch string letter
    (:a
      (Niagara|SetTextureObject (Variables|NiagaraActor|GetNiagaraComponent) "user.Alphabet" "/Game/p3/VFX/alphabet_texture/a.a"))
    (:b
      (Niagara|SetTextureObject (Variables|NiagaraActor|GetNiagaraComponent) "user.Alphabet" "/Game/p3/VFX/alphabet_texture/b.b"))
    (:c
      (Niagara|SetTextureObject (Variables|NiagaraActor|GetNiagaraComponent) "user.Alphabet" "/Game/p3/VFX/alphabet_texture/c.c"))
    (:d
      (Niagara|SetTextureObject (Variables|NiagaraActor|GetNiagaraComponent) "user.Alphabet" "/Game/p3/VFX/alphabet_texture/d.d"))
    (:e
      (Niagara|SetTextureObject (Variables|NiagaraActor|GetNiagaraComponent) "user.Alphabet" "/Game/p3/VFX/alphabet_texture/e.e"))
    (:f
      (Niagara|SetTextureObject (Variables|NiagaraActor|GetNiagaraComponent) "user.Alphabet" "/Game/p3/VFX/alphabet_texture/f.f"))
    (:g
      (Niagara|SetTextureObject (Variables|NiagaraActor|GetNiagaraComponent) "user.Alphabet" "/Game/p3/VFX/alphabet_texture/g.g"))
    (:h
      (Niagara|SetTextureObject (Variables|NiagaraActor|GetNiagaraComponent) "user.Alphabet" "/Game/p3/VFX/alphabet_texture/h.h"))
    (:i
      (Niagara|SetTextureObject (Variables|NiagaraActor|GetNiagaraComponent) "user.Alphabet" "/Game/p3/VFX/alphabet_texture/i.i"))
    (:j
      (Niagara|SetTextureObject (Variables|NiagaraActor|GetNiagaraComponent) "user.Alphabet" "/Game/p3/VFX/alphabet_texture/j.j"))
    (:k
      (Niagara|SetTextureObject (Variables|NiagaraActor|GetNiagaraComponent) "user.Alphabet" "/Game/p3/VFX/alphabet_texture/k.k"))
    (:l
      (Niagara|SetTextureObject (Variables|NiagaraActor|GetNiagaraComponent) "user.Alphabet" "/Game/p3/VFX/alphabet_texture/l.l"))
    (:m
      (Niagara|SetTextureObject (Variables|NiagaraActor|GetNiagaraComponent) "user.Alphabet" "/Game/p3/VFX/alphabet_texture/m.m"))
    (:n
      (Niagara|SetTextureObject (Variables|NiagaraActor|GetNiagaraComponent) "user.Alphabet" "/Game/p3/VFX/alphabet_texture/n.n"))
    (:o
      (Niagara|SetTextureObject (Variables|NiagaraActor|GetNiagaraComponent) "user.Alphabet" "/Game/p3/VFX/alphabet_texture/o.o"))
    (:p
      (Niagara|SetTextureObject (Variables|NiagaraActor|GetNiagaraComponent) "user.Alphabet" "/Game/p3/VFX/alphabet_texture/p.p"))
    (:q
      (Niagara|SetTextureObject (Variables|NiagaraActor|GetNiagaraComponent) "user.Alphabet" "/Game/p3/VFX/alphabet_texture/q.q"))
    (:r
      (Niagara|SetTextureObject (Variables|NiagaraActor|GetNiagaraComponent) "user.Alphabet" "/Game/p3/VFX/alphabet_texture/r.r"))
    (:s
      (Niagara|SetTextureObject (Variables|NiagaraActor|GetNiagaraComponent) "user.Alphabet" "/Game/p3/VFX/alphabet_texture/s.s"))
    (:t
      (Niagara|SetTextureObject (Variables|NiagaraActor|GetNiagaraComponent) "user.Alphabet" "/Game/p3/VFX/alphabet_texture/t.t"))
    (:u
      (Niagara|SetTextureObject (Variables|NiagaraActor|GetNiagaraComponent) "user.Alphabet" "/Game/p3/VFX/alphabet_texture/u.u"))
    (:v
      (Niagara|SetTextureObject (Variables|NiagaraActor|GetNiagaraComponent) "user.Alphabet" "/Game/p3/VFX/alphabet_texture/v.v"))
    (:w
      (Niagara|SetTextureObject (Variables|NiagaraActor|GetNiagaraComponent) "user.Alphabet" "/Game/p3/VFX/alphabet_texture/w.w"))
    (:x
      (Niagara|SetTextureObject (Variables|NiagaraActor|GetNiagaraComponent) "user.Alphabet" "/Game/p3/VFX/alphabet_texture/x.x"))
    (:y
      (Niagara|SetTextureObject (Variables|NiagaraActor|GetNiagaraComponent) "user.Alphabet" "/Game/p3/VFX/alphabet_texture/y.y"))
    (:z
      (Niagara|SetTextureObject (Variables|NiagaraActor|GetNiagaraComponent) "user.Alphabet" "/Game/p3/VFX/alphabet_texture/z.z"))))