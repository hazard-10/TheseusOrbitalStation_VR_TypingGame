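; BP_demon is an enemy actor that advances on the heart and drains its HP.
; On BeginPlay it caches the first actor tagged "heart" as a BP_heart reference.
; Each Tick it steps straight toward the heart by a fixed per-frame offset, without sweep or delta-time scaling, until within StopDistance.
; Once in range, a delta-time accumulator removes one HP from the heart each time it reaches MaxTime, then resets.
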(event EventBeginPlay
  (bind _outactors (Actor|GetAllActorswithTag "heart"))
  (bind _asbp_heart (Utilities|Casting|CastToBP_heart (Utilities|Array|Get(acopy) _outactors)))
  (Variables|Default|Setheart_reference _asbp_heart))

(event EventTick
  (params (DeltaSeconds :type Float%20%28single-precision%29))
  (bind _heart_reference (Variables|Default|Getheart_reference))
  (if (> (Transformation|GetDistanceTo (Variables|Default|Getheart_reference)) (Variables|Default|Getstop_distance))
    (Transformation|AddActorWorldOffset (* (Math|Vector|GetUnitDirection(Vector) (Transformation|GetActorLocation) (Transformation|GetActorLocation (Variables|Default|Getheart_reference))) "2.000000,2.000000,2.000000"))
    (else
      (bind _output_get (Variables|Default|Settime (+ (Variables|Default|Gettime) (Utilities|Time|GetWorldDeltaSeconds))))
      (if (>= _output_get (Variables|Default|Getmax_time))
        (Variables|Default|Settime 0.0)
        (Variables|/Game/p3/heart/BP_heart.BP_heart_C|Sethp _heart_reference (- (Variables|/Game/p3/heart/BP_heart.BP_heart_C|Gethp _heart_reference) 1))))))

(fn ConstructionScript)