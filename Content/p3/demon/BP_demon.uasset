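; BP_demon is an enemy that chases the heart actor and drains its HP, with a word displayed above it.
; It finds the heart by tag on BeginPlay, then each Tick moves straight toward it unless the game is stopped.
; Within stop distance, it removes one HP at a timed interval.
; UpdateHitEffect maps Progress to a Dissolve parameter on a dynamic material instance, but is not called here.
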(event EventBeginPlay
  (bind _outactors (Actor|GetAllActorswithTag "heart"))
  (bind _asbp_heart (Utilities|Casting|CastToBP_heart (Utilities|Array|Get(acopy) _outactors)))
  (Variables|Default|Setheart_reference _asbp_heart))

(event EventTick
  (params (DeltaSeconds :type Float%20%28single-precision%29))
  (bind _heart_reference (Variables|Default|Getheart_reference))
  ;[1 1 1] Set the text above demon's head
  (CallFunction|SetDemonText)
  (if (> (Transformation|GetDistanceTo (Variables|Default|Getheart_reference)) (Variables|Default|Getstop_distance))
    (if (not (Variables|Default|Getgame_is_stoppped))
      (Transformation|AddActorWorldOffset (* (Math|Vector|GetUnitDirection(Vector) (Transformation|GetActorLocation) (Transformation|GetActorLocation (Variables|Default|Getheart_reference))) (Variables|Default|Getspeed))))
    (else
      (bind _output_get (Variables|Default|Settime (+ (Variables|Default|Gettime) (Utilities|Time|GetWorldDeltaSeconds))))
      (if (>= _output_get (Variables|Default|Getmax_time))
        (Variables|Default|Settime 0.0)
        (Variables|/Game/p3/heart/BP_heart.BP_heart_C|Sethp _heart_reference (- (Variables|/Game/p3/heart/BP_heart.BP_heart_C|Gethp _heart_reference) 1))))))

(fn ConstructionScript)

(fn SetDemonText
  (bind _asarrow_widget (Utilities|Casting|CastToArrowWidget (UserInterface|GetUserWidgetObject (Variables|Default|GetDemonText))))
  (Default|SpawnNewString _asarrow_widget (Variables|Default|Getword)))

(fn UpdateHitEffect
  (bind _returnvalue (Rendering|Material|CreateDynamicMaterialInstance (Variables|Debug|GetStaticMeshComponent) 0 "/Game/p3/demon/cube_placeholder/asteroid/asteroid_MAT.asteroid_MAT" "None" :!class /Script/Engine.PrimitiveComponent))
  (Rendering|Material|SetScalarParameterValue _returnvalue "Dissolve" (/ (- 1.0 (Variables|Default|Getprogress)) 2.0) :!class /Script/Engine.MaterialInstanceDynamic))